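; BP_CustomClothSim is a placeable custom cloth simulation that exposes panel size and spring tuning on each instance.
; BeginPlay builds the cloth from those dimensions and structural, shear and flex spring settings, then enables cloth collision.
; Each Tick steps the simulation with PlayerVel as outside force, then resets PlayerVel to a small random uniform vector for the next frame.
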(event `self.ReceiveBeginPlay`
  ; On Begin Play Set up Cloth Sim
  (`self.SetClothSim` (`self.Width`) (`self.Hight`) (`self.PanelSize`) (`self.Struct Spring Kd`) (`self.Struct Spring Ks`) (`self.Shear Spring Kd`) (`self.Shear Spring Ks`) (`self.Flex Spring Kd`) (`self.Flex Spring Ks`))
  (`self.EnableClothCollision`))

(event `self.ReceiveTick`
  (params (DeltaSeconds :type "Float (single-precision)"))
  ; Update Cloth every event tick - if player is colliding on event tick add player velocity to the cloth
  (`self.ClothTick` DeltaSeconds (stale _output_get))
  (bind _output_get (set `self.PlayerVel` (`KismetMathLibrary.Conv_DoubleToVector` (`KismetMathLibrary.RandomFloatInRange` 0.0 20.0)))))

(fn `UserConstructionScript`)